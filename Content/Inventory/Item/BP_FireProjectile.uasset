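; BP_FireProjectile is an inventory item actor that sets the player's projectile selection when interacted with, presumably to a fire projectile.
; Interact destroys the actor, casts player 0's character to BP_Character, sets its Projectile value and returns the item's SItemData.
; The event graph holds only disabled default events, and the construction script just calls its parent.
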(event EventBeginPlay
  (|CallParentFunction) ; This node is disabled and will not be called.\nDrag off pins to build functionality.
)

(event Collision|EventActorBeginOverlap
  (params (OtherActor :type Actor%20Object%20Reference))
  (|CallParentFunction OtherActor) ; This node is disabled and will not be called.\nDrag off pins to build functionality.
)

(event EventTick
  (params (DeltaSeconds :type Float%20%28single-precision%29))
  (|CallParentFunction DeltaSeconds) ; This node is disabled and will not be called.\nDrag off pins to build functionality.
)

(fn ConstructionScript
  (|CallParentFunction))

(fn Interact
  (Actor|DestroyActor)
  (bind _asbp_character (Utilities|Casting|CastToBP_Character (Game|GetPlayerCharacter 0)))
  (Variables|/Game/BluePrint/BP_Character.BP_Character_C|SetProjectile _asbp_character 1)
  (return (Variables|Default|GetS_ItemData)))